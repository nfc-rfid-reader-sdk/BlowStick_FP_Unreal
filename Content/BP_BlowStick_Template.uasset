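; BP_BlowStick_Template is a template for using BlowStick controller input, displaying its live readings in a debug stats widget.
; On BeginPlay it finds the BP_BlowStick_Controller, binds to its blow-action dispatcher, shows the mouse and creates the UI.
; Tick treats non-zero rotation as connected, updating status, rotation and blow values, with no reset to disconnected.
; Dispatched blows pass through BlowActionEvent, which displays the last blow power.
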(event `self.ReceiveBeginPlay`
  ;[1 1 1] Add BlowStick Controller
  (bind _outactors (`GameplayStatics.GetAllActorsOfClass` "/Game/blowstick-bp-unreal/BP_BlowStick_Controller.BP_BlowStick_Controller_C"))
  (bind _output_get (set `self.BlowStick_Controller` (`|GetArrayItem` _outactors)))
  ;[1 1 1] Bind Event BlowAction
  (add `/Game/blowstick-bp-unreal/BP_BlowStick_Controller.BlowActionEventDispatcher` _output_get (delegate `BlowActionReceiver`))
  ;[1 1 1] Show Mouse
  (set `PlayerController.bShowMouseCursor` true (`GameplayStatics.GetPlayerController` 0))
  ;[1 1 1] Get BlowStic UI and add it to Viewport
  (bind _returnvalue (`|CreateWidget` "/Game/UI_BlowStickStats.UI_BlowStickStats_C" (`GameplayStatics.GetPlayerController` 0)))
  (bind _output_get_2 (set `self.BlowStick_Stats` _returnvalue))
  (`UserWidget.AddToViewport` _output_get_2 0))

(event `BlowActionReceiver`
  (params (BlowPower :type "Float (double-precision)"))
  ;[1 1 1] Bind Event BlowAction
  (`self.BlowActionEvent` BlowPower))

(event `self.ReceiveTick`
  (params (DeltaSeconds :type "Float (single-precision)"))
  (bind _blowstick_controller (`self.BlowStick_Controller`))
  (bind _connectionstatus (`/Game/UI_BlowStickStats.ConnectionStatus` (`self.BlowStick_Stats`)))
  (bind (_blowstick_rotator_roll _blowstick_rotator_pitch _blowstick_rotator_yaw) (`KismetMathLibrary.BreakRotator` (`/Game/blowstick-bp-unreal/BP_BlowStick_Controller.BlowStick_Rotator` _blowstick_controller)))
  ;[1 1 1] Fill BlowStick Status UI
  (if (!= (`/Game/blowstick-bp-unreal/BP_BlowStick_Controller.BlowStick_Rotator` (`self.BlowStick_Controller`)) (struct) :`ErrorTolerance` 0.0)
    (`TextBlock.SetText` _connectionstatus "Connected")
    (`TextBlock.SetColorAndOpacity` _connectionstatus (make `SlateColor` (struct :`G` 1.0 :`B` 0.12332 :`A` 1.0)))
    (`TextBlock.SetText` (`/Game/UI_BlowStickStats.BlowStickRoll` (`self.BlowStick_Stats`)) (`KismetTextLibrary.Conv_DoubleToText` _blowstick_rotator_roll "HalfToEven"))
    (`TextBlock.SetText` (`/Game/UI_BlowStickStats.BlowStickPitch` (`self.BlowStick_Stats`)) (`KismetTextLibrary.Conv_DoubleToText` _blowstick_rotator_pitch "HalfToEven"))
    (`TextBlock.SetText` (`/Game/UI_BlowStickStats.BlowStickYaw` (`self.BlowStick_Stats`)) (`KismetTextLibrary.Conv_DoubleToText` _blowstick_rotator_yaw "HalfToEven"))
    (`TextBlock.SetText` (`/Game/UI_BlowStickStats.BlowStickBlowAction` (`self.BlowStick_Stats`)) (`KismetTextLibrary.Conv_DoubleToText` (`/Game/blowstick-bp-unreal/BP_BlowStick_Controller.BlowStick_Blow_Action` _blowstick_controller) "HalfToEven"))
    (`TextBlock.SetText` (`/Game/UI_BlowStickStats.BlowStickBlowPowerInertialised` (`self.BlowStick_Stats`)) (`KismetTextLibrary.Conv_DoubleToText` (`/Game/blowstick-bp-unreal/BP_BlowStick_Controller.BlowStick_Blow_Inertialised` _blowstick_controller) "HalfToEven"))
    (`TextBlock.SetText` (`/Game/UI_BlowStickStats.BlowStickBlowPowerRaw` (`self.BlowStick_Stats`)) (`KismetTextLibrary.Conv_DoubleToText` (`/Game/blowstick-bp-unreal/BP_BlowStick_Controller.BlowStick_Blow_Raw` _blowstick_controller) "HalfToEven"))))

(event `BlowActionEvent`
  (params (BlowPower :type "Float (double-precision)"))
  ;[1 1 1] Fill BlowStick Status UI
  (`TextBlock.SetText` (`/Game/UI_BlowStickStats.BlowStickLastBlowAction` (`self.BlowStick_Stats`)) (`KismetTextLibrary.Conv_DoubleToText` BlowPower "HalfToEven")))

(fn `UserConstructionScript`)